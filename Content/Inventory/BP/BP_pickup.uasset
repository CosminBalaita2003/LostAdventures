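; World inventory pickup actor that bobs on a timeline and lets a nearby character collect it with E.
; The ID's RepNotify, also run at construction and BeginPlay, resolves item data from DT_Inventory or a DropItem override, then updates the widget text and blocking-loads the mesh.
; Sphere overlap toggles the widget and player 0's input.
; Pressing E sends the item to the character and destroys the actor on success.
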(event OnComponentBeginOverlap(Sphere)
  (params (OverlappedComponent :type Primitive%20Component%20Object%20Reference) (OtherActor :type Actor%20Object%20Reference) (OtherComp :type Primitive%20Component%20Object%20Reference) (OtherBodyIndex :type Integer) (bFromSweep :type Boolean) (SweepResult :type Hit%20Result%20Structure%20%28by%20ref%29))
  ;[1 1 1] overlap - show widget when player overlaps with Sphere
  (Rendering|SetVisibility (Variables|Default|GetWidget) true false)
  ;[1 0.1575 0.4441] Allow interaction
  (Input|EnableInput (Game|GetPlayerController 0))
  (bind _ascharacter (Utilities|Casting|CastToCharacter OtherActor))
  (Variables|Default|SetCharacter _ascharacter))

(event OnComponentEndOverlap(Sphere)
  (params (OverlappedComponent :type Primitive%20Component%20Object%20Reference) (OtherActor :type Actor%20Object%20Reference) (OtherComp :type Primitive%20Component%20Object%20Reference) (OtherBodyIndex :type Integer))
  ;[1 1 1] overlap - show widget when player overlaps with Sphere
  (Rendering|SetVisibility (Variables|Default|GetWidget) false false)
  ;[1 0.1575 0.4441] Allow interaction
  (Input|DisableInput (Game|GetPlayerController 0)))

(event Custom|Update
  (bind _item (Variables|Default|GetItem))
  (bind (_displayname _pickupmeshstatic) (Utilities|Struct|BreakST_Inventory_item _item))
  ;[1 1 1] Display widget
  (bind _aswp_pickup (Utilities|Casting|CastTowp_pickup (UserInterface|GetWidget (Variables|Default|GetWidget))))
  (Variables|/Script/UMG.TextBlock|SetText (Variables|/Game/Inventory/Widget/wp_pickup.wp_pickup_C|GetText _aswp_pickup) _displayname)
  (bind _returnvalue (Utilities|LoadAssetBlocking _pickupmeshstatic))
  (bind _asstatic_mesh (Utilities|Casting|CastToStaticMesh _returnvalue))
  (Components|StaticMesh|SetStaticMesh (Variables|Default|GetStaticMesh) _asstatic_mesh))

(event EventBeginPlay
  (bind _returnvalue (Transformation|GetActorLocation))
  (bind (_x _y _z) (Math|Vector|BreakVector _returnvalue))
  ;[1 1 1] Floating
  (CallFunction|OnRepID)
  (bind _height (Timeline|Plutire PlayFromStart)
    (:Update
      (Transformation|SetActorLocation (Math|Vector|MakeVector _x _y (+ (* _height (Math|Random|RandomFloatinRange 1.0 5.0)) _z)) false false))))

(event Input|KeyboardEvents|E
  (params (Key :type Key%20Structure :default "None"))
  (:Pressed
    (bind _succes (Class|BPIInventory|PickUpItem(Message) (Variables|Default|GetCharacter) (Variables|Default|GetID) (Variables|Default|GetItem)))
    (if _succes
      (Actor|DestroyActor))))

(fn ConstructionScript
  (CallFunction|OnRepID))

(fn OnRepID
  (bind _returnvalue (Utilities|GetDataTableRow "/Game/Inventory/DT_Inventory.DT_Inventory" (Variables|Default|GetID))
    (:then
      (Variables|Default|SetItem (select (!= (Utilities|Struct|BreakST_Inventory_item (Variables|Default|GetDropItem)) "") (Variables|Default|GetDropItem) _returnvalue))
      (CallFunction|Update))))