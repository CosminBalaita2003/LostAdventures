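; Inventory component with a Give function that adds an item to the Items map by ID.
; The ID must exist in DT_Inventory or Give returns false; a valid DropItem overrides the table row's data, and a Quantity other than -1 overrides its count.
; Items already held have their quantity increased, while new ones are added as fresh entries, both returning true.
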(fn Give
  (params (ID :type Name) (Quantity :type Integer) (DropItem :type ST%20Inventory%20Item%20Structure))
  (bind _items (Variables|Default|GetItems))
  (bind (_value _returnvalue) (Utilities|Map|Find _items ID))
  (Utilities|FlowControl|Sequence
    (:then_0
      ;[1 1 1] Check item exists
      (bind _returnvalue_2 (Utilities|GetDataTableRow "/Game/Inventory/DT_Inventory.DT_Inventory" ID)
        (:then
          (bind _output_get (LocalVariables|SetItem (select (!= (.ID (Utilities|Struct|BreakST_Inventory_item DropItem)) "") DropItem _returnvalue_2)))
          (if (!= Quantity -1)
            (bind _structout (Utilities|Struct|SetmembersinST_Inventory_item _output_get Quantity))
            (LocalVariables|SetItem _structout)))
        (:RowNotFound
          (return false))))
    (:then_1
      ;[1 1 1] Check player has item
      (if _returnvalue
        (bind _structout_2 (Utilities|Struct|SetmembersinST_Inventory_item _value (+ (Utilities|Struct|BreakST_Inventory_item _value) (Utilities|Struct|BreakST_Inventory_item (LocalVariables|GetItem)))))
        (Utilities|Map|Add (Variables|Default|GetItems) ID _structout_2)
        (return true)))
    (:then_2
      ;[1 1 1] Add item to inventory
      (Utilities|Map|Add (Variables|Default|GetItems) ID (LocalVariables|GetItem))
      (return true))))